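; BP_Ship is a ship actor that travels along a RouteSpline found in the level while rocking its hull.
; A rate-scaled MoveObjectT timeline drives location and rotation from distance along the spline.
; The Sailing timeline tilts the body mesh, reverses and restarts itself, with random pitch and roll amplitudes via a DoOnce.
; Key 1 also swaps the streamed Day level for DayNight.
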(event Custom|Move
  (bind _splineref (Variables|Default|GetSplineRef))
  (bind _spline (Variables|/Game/RouteSpline.RouteSpline_C|GetSpline _splineref))
  (Components|Timeline|SetPlayRate (Variables|Default|GetMove%20Object%20T) (/ 1.0 (Variables|Default|GetTimeComplete)))
  (bind _move (Timeline|Move%20Object%20T Play)
    (:Update
      (Transformation|SetActorTransform (Math|Transform|MakeTransform (Spline|GetLocationatDistanceAlongSpline _spline (Math|Float|Lerp 0.0 (Spline|GetSplineLength (Variables|/Game/RouteSpline.RouteSpline_C|GetSpline (Variables|Default|GetSplineRef))) _move) "World") (Spline|GetRotationatDistanceAlongSpline _spline (Math|Float|Lerp 0.0 (Spline|GetSplineLength (Variables|/Game/RouteSpline.RouteSpline_C|GetSpline (Variables|Default|GetSplineRef))) _move) "Local") "1.000000,1.000000,1.000000")))))

(event Custom|Sail
  (Utilities|FlowControl|Sequence
    (:then_0
      (bind _sailing (Timeline|Sailing Play)
        (:Update
          (Transformation|SetRelativeRotation (Variables|Default|GetSM_ShipMainBody_00) (Math|Rotator|MakeRotator (Math|Float|Lerp 0.0 (Variables|Default|GetYPitch) _sailing) (Math|Float|Lerp 0.0 (Variables|Default|GetXRoll) _sailing) 0.0) false false))
        (:Finished
          (CallFunction|Reverse)
          (Utilities|FlowControl|Delay 1.5)
          (if (Variables|Default|GetIsRev)
            (Variables|Default|SetIsRev false)
            (CallFunction|Sail)
            (goto _label Reset)))))
    (:then_1
      (if (not (Variables|Default|GetIsRev))
        (Utilities|FlowControl|DoOnce false :!label _label
          (:Completed
            (Variables|Default|SetYPitch (Math|Random|RandomFloatinRange -0.5 0.5))
            (Variables|Default|SetXRoll (Math|Random|RandomFloatinRange -2.0 2.0))))))))

(event Custom|Reverse
  (Variables|Default|SetIsRev true)
  (bind _sailing (Timeline|Sailing Reverse)
    (:Update
      (Transformation|SetRelativeRotation (Variables|Default|GetSM_ShipMainBody_00) (Math|Rotator|MakeRotator (Math|Float|Lerp 0.0 (Variables|Default|GetYPitch) _sailing) (Math|Float|Lerp 0.0 (Variables|Default|GetXRoll) _sailing) 0.0) false false))
    (:Finished
      (CallFunction|Reverse)
      (Utilities|FlowControl|Delay 1.5)
      (if (Variables|Default|GetIsRev)
        (Variables|Default|SetIsRev false)
        (CallFunction|Sail)
        (Utilities|FlowControl|DoOnce false) ; enters at Reset
      ))))

(event EventBeginPlay
  (bind _outactors (Actor|GetAllActorsOfClass "/Game/RouteSpline.RouteSpline_C"))
  (for _array_element _outactors
    (Variables|Default|SetSplineRef _array_element)
    (CallFunction|Move)
    (CallFunction|Sail)))

(event Input|KeyboardEvents|1
  (params (Key :type Key%20Structure :default "None"))
  (:Pressed
    (Game|LoadStreamLevel(byName) "DayNight" true)
    (Game|UnloadStreamLevel(byName) "Day" false))
  (:Released
    (Game|UnloadStreamLevel(byName) "Day" false)
    (Game|LoadStreamLevel(byName) "DayNight" true)))

(fn ConstructionScript)